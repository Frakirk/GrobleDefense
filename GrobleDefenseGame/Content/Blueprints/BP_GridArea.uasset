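; BP_GridArea builds a grid of ground-projected transforms inside its Box bounds.
; GenerateGridTransforms snaps the box center up to GridScale multiples with RoundVector, then loops over X and Y cells sized by that scale.
; Each cell traces vertically through the box against WorldStatic with debug drawing, storing the impact point in GridTransforms without checking for a hit.
; Event graph and construction script are empty, so nothing here triggers generation.
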(fn `GenerateGridTransforms`
  (locals (TraceStart :type "Vector Structure") (TraceEnd :type "Vector Structure") (RoundedBounds :type "Vector Structure") (BoundsHeight :type "Float (double-precision)") (RoundedOrigin :type "Vector Structure") (GridXPos :type "Float (double-precision)") (GridYPos :type "Float (double-precision)") (OriginZPos :type "Float (double-precision)") (OutputTransforms :type "Array of Transform Structure"))
  (bind (_roundedorigin_x _roundedorigin_y) (`KismetMathLibrary.BreakVector` (`local.RoundedOrigin`)))
  (bind (_origin _boxextent) (`KismetSystemLibrary.GetComponentBounds` (`self.Box`)))
  (bind _returnvalue (`KismetMathLibrary.FFloor` (/ (.y _boxextent) (`KismetMathLibrary.Conv_IntToDouble` (`self.GridScale`)))))
  (bind _returnvalue_2 (`KismetMathLibrary.FFloor` (/ (.x _boxextent) (`KismetMathLibrary.Conv_IntToDouble` (`self.GridScale`)))))
  (set `local.OriginZPos` (.z _origin))
  (set `local.RoundedOrigin` (`self.RoundVector` _origin (`self.GridScale`)))
  (set `local.BoundsHeight` (.z _boxextent))
  (for _index (range (- (* _returnvalue_2 -1) 1) _returnvalue_2)
    (for _index_2 (range (- (* _returnvalue -1) 1) _returnvalue)
      (set `local.GridXPos` (+ (`KismetMathLibrary.Conv_IntToDouble` (* _index (`self.GridScale`))) _roundedorigin_x))
      (set `local.GridYPos` (+ (`KismetMathLibrary.Conv_IntToDouble` (* _index_2 (`self.GridScale`))) _roundedorigin_y))
      (set `local.TraceStart` (`KismetMathLibrary.MakeVector` (`local.GridXPos`) (`local.GridYPos`) (+ (`local.OriginZPos`) (`local.BoundsHeight`))))
      (set `local.TraceEnd` (`KismetMathLibrary.MakeVector` (`local.GridXPos`) (`local.GridYPos`) (- (`local.OriginZPos`) (`local.BoundsHeight`))))
      (bind _outhit (`KismetSystemLibrary.LineTraceSingleForObjects` :`Start` (`local.TraceStart`) :`End` (`local.TraceEnd`) :`ObjectTypes` (`|MakeArray` (enumliteral `EObjectTypeQuery` "ObjectTypeQuery1")) :`DrawDebugType` "ForDuration"))
      (`KismetArrayLibrary.Array_Add` (`local.OutputTransforms`) (`KismetMathLibrary.MakeTransform` (`.ImpactPoint` (`GameplayStatics.BreakHitResult` _outhit)) (struct) (1.0 1.0 1.0)))))
  (set `self.GridTransforms` (`local.OutputTransforms`)))

(fn `RoundVector`
  (params (Input :type "Vector Structure") (RoundingFactor :type Integer))
  (returns (Output :type "Vector Structure"))
  (return (`KismetMathLibrary.MakeVector` (`KismetMathLibrary.Conv_IntToDouble` (* (`KismetMathLibrary.FCeil` (.x (/ Input RoundingFactor))) (`local.RoundingFactor`))) (`KismetMathLibrary.Conv_IntToDouble` (* (`KismetMathLibrary.FCeil` (.y (/ Input RoundingFactor))) (`local.RoundingFactor`))) (`KismetMathLibrary.Conv_IntToDouble` (* (`KismetMathLibrary.FCeil` (.z (/ Input RoundingFactor))) (`local.RoundingFactor`))))))

(fn `UserConstructionScript`)