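; BP_Creep is an enemy that walks toward a target exit portal, re-issuing a simple AI move every two seconds.
; Construction scales max hit points by Level.
; UpdateHealth applies signed deltas to the health bar widget and, at zero or below, spawns BP_Gold carrying its GoldValue before destroying the creep.
; Tick bobs the billboard on a sine wave and yaws the health bar toward the camera.
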(event `NavigateToExit`
  (`AIBlueprintHelperLibrary.SimpleMoveToActor` (`self.GetController`) (`self.TargetExitPortal`))
  (`KismetSystemLibrary.Delay` 2.0)
  (`self.NavigateToExit`))

(event `self.ReceiveBeginPlay`
  (bind _asw_health_bar (cast `/Game/Widgets/W_HealthBar` (`WidgetComponent.GetWidget` (`self.HealthbarWidget`))))
  (set `self.Healthbar` _asw_health_bar)
  (`self.Update Health` 0.0)
  (`self.NavigateToExit`))

(event `self.ReceiveTick`
  (params (DeltaSeconds :type "Float (single-precision)"))
  (bind (_returnvalue_roll _returnvalue_pitch _returnvalue_yaw) (`KismetMathLibrary.BreakRotator` (`KismetMathLibrary.FindLookAtRotation` (`SceneComponent.K2_GetComponentLocation` (`self.HealthbarWidget`)) (`PlayerCameraManager.GetCameraLocation` (`GameplayStatics.GetPlayerCameraManager` 0)))))
  (bind _output_get (set `self.Age` (+ (`self.Age`) DeltaSeconds)))
  (`SceneComponent.K2_SetRelativeLocation` (`self.Billboard`) (`KismetMathLibrary.MakeVector` 0.0 0.0 (+ (* (`KismetMathLibrary.Sin` _output_get) 50.0) 100.0)) false false)
  (`SceneComponent.K2_SetWorldRotation` (`self.HealthbarWidget`) (`KismetMathLibrary.MakeRotator` 0.0 0.0 _returnvalue_yaw) false false))

(fn `Update Health`
  (params (HealthDelta :type "Float (double-precision)"))
  (set `self.HitPointsCurrent` (+ HealthDelta (`self.HitPointsCurrent`)))
  (`/Game/Widgets/W_HealthBar.UpdateHealthPercentage` (`self.Healthbar`) (/ (`self.HitPointsCurrent`) (`self.HitPointsMax`)))
  (if (>= 0.0 (`self.HitPointsCurrent`))
    (`|SpawnActorFromClass` "/Game/Blueprints/BP_Gold.BP_Gold_C" (`KismetMathLibrary.MakeTransform` (`self.K2_GetActorLocation`)) "AdjustIfPossibleButAlwaysSpawn" "OverrideRootScale" null (`self.GoldValue`) null)
    (`self.K2_DestroyActor`)))

(fn `UserConstructionScript`
  (bind _hitpointsmax (`self.HitPointsMax`))
  (set `self.HitPointsMax` (+ _hitpointsmax (* _hitpointsmax (* (`self.Level`) 0.5))))
  (set `self.HitPointsCurrent` (`self.HitPointsMax`)))