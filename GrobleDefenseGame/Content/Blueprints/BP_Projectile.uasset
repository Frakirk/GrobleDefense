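; BP_Projectile is a homing projectile that damages or otherwise changes the health of the creep it hits.
; On BeginPlay it registers with its target's TargetingProjectiles list and homes on that target's ProjectileTarget component.
; A spawn timeline scales the actor up while ramping homing acceleration from the same curve.
; Overlapping any BP_Creep with its sphere applies HealthDelta and destroys the projectile.
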(event `self.ReceiveBeginPlay`
  (`KismetArrayLibrary.Array_Add` (`/Game/Blueprints/BP_Creep.TargetingProjectiles` (`self.Target`)) self)
  (set `self.HomingAcceleration` (`ProjectileMovementComponent.HomingAccelerationMagnitude` (`self.ProjectileMovement`)))
  (set `ProjectileMovementComponent.HomingTargetComponent` (`/Game/Blueprints/BP_Creep.ProjectileTarget` (`self.Target`)) (`self.ProjectileMovement`))
  (bind (_direction _scale) (`Timeline|ProjectileSpawn` :!via `PlayFromStart`)
    (:`Update`
      (`self.SetActorScale3D` (`KismetMathLibrary.Conv_DoubleToVector` _scale))
      (set `ProjectileMovementComponent.HomingAccelerationMagnitude` (* _scale (`self.HomingAcceleration`)) (`self.ProjectileMovement`)))))

(event `self.Sphere1.OnComponentBeginOverlap`
  (params (OverlappedComponent :type "PrimitiveComponent Object Reference") (OtherActor :type "Actor Object Reference") (OtherComp :type "PrimitiveComponent Object Reference") (OtherBodyIndex :type Integer) (bFromSweep :type Boolean) (SweepResult :type "HitResult Structure (by ref)"))
  (bind _asbp_creep (cast `/Game/Blueprints/BP_Creep` OtherActor))
  (`/Game/Blueprints/BP_Creep.Update Health` _asbp_creep (`self.HealthDelta`))
  (`self.K2_DestroyActor`))

(fn `UserConstructionScript`)