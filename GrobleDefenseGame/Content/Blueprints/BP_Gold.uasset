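; Gold actor with a Cube component whose world size reflects its GoldValue.
; The construction script scales the cube uniformly to a tenth of GoldValue.
; On BeginPlay the cube is launched in a random direction with a mass-independent impulse, scattering the gold as it spawns.
; The Blueprint contains no collection or overlap logic.
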(event `self.ReceiveBeginPlay`
  (`PrimitiveComponent.AddImpulse` (`self.Cube`) (* (`KismetMathLibrary.RandomUnitVector`) 500.0) "None" true))

(fn `UserConstructionScript`
  (`SceneComponent.SetWorldScale3D` (`self.Cube`) (`KismetMathLibrary.Conv_DoubleToVector` (/ (`KismetMathLibrary.Conv_IntToDouble` (`self.GoldValue`)) 10.0))))