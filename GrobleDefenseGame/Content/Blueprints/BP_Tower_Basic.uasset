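; BP_Tower_Basic is a tower Blueprint that sizes its Capsule component according to its Level.
; The construction script calls the parent's script, then sets both capsule half-height and radius from the same linear formula on Level, so the volume becomes a sphere that grows with each level.
; The event graph holds only disabled default events, so the Blueprint adds no runtime logic of its own.
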(fn `UserConstructionScript`
  (bind _returnvalue (`KismetMathLibrary.Conv_IntToDouble` (+ (* (- (`self.Level`) 1) 200) 300)))
  (`parent.UserConstructionScript`)
  (`CapsuleComponent.SetCapsuleHalfHeight` (`self.Capsule`) _returnvalue true)
  (`CapsuleComponent.SetCapsuleRadius` (`self.Capsule`) _returnvalue true))