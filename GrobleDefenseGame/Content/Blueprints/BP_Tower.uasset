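; BP_Tower is a tower that fires projectiles at creeps inside its capsule trigger, which the construction script sizes by Level.
; Capsule overlaps maintain a creep list, and a creep entering while off cooldown triggers an attack.
; Attack spawns the projectile aimed at the most recently added creep and resets the cooldown.
; Rather than using Tick, TickCooldown re-calls itself through zero-second delays until ready, then attacks again if creeps remain.
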(event `TickCooldown`
  (bind _output_get (set `self.AttackCooldown` (- (`self.AttackCooldown`) (`GameplayStatics.GetWorldDeltaSeconds`))))
  (if (<= _output_get 0.0)
    (set `self.AttackCooldown` 0.0)
    (if (> (`KismetArrayLibrary.Array_Length` (`self.CreepsInRange`)) 0)
      (`self.Attack`))
    (else
      (`KismetSystemLibrary.Delay` 0.0)
      (`self.TickCooldown`))))

(event `self.Capsule.OnComponentBeginOverlap`
  (params (OverlappedComponent :type "PrimitiveComponent Object Reference") (OtherActor :type "Actor Object Reference") (OtherComp :type "PrimitiveComponent Object Reference") (OtherBodyIndex :type Integer) (bFromSweep :type Boolean) (SweepResult :type "HitResult Structure (by ref)"))
  (bind _asbp_creep (cast `/Game/Blueprints/BP_Creep` OtherActor))
  (`KismetArrayLibrary.Array_AddUnique` (`self.CreepsInRange`) _asbp_creep)
  (if (<= (`self.AttackCooldown`) 0.0)
    (`self.Attack`)))

(event `self.Capsule.OnComponentEndOverlap`
  (params (OverlappedComponent :type "PrimitiveComponent Object Reference") (OtherActor :type "Actor Object Reference") (OtherComp :type "PrimitiveComponent Object Reference") (OtherBodyIndex :type Integer))
  (bind _asbp_creep (cast `/Game/Blueprints/BP_Creep` OtherActor))
  (`KismetArrayLibrary.Array_RemoveItem` (`self.CreepsInRange`) _asbp_creep))

(fn `Attack`
  (bind _creepsinrange (`self.CreepsInRange`))
  (`|SpawnActorFromClass` (`self.AttackProjectile`) (`KismetMathLibrary.MakeTransform` (`SceneComponent.K2_GetComponentLocation` (`self.AttackOrigin`))) "Undefined" "OverrideRootScale" self (`|GetArrayItem` _creepsinrange (`KismetArrayLibrary.Array_LastIndex` _creepsinrange)) null)
  (set `self.AttackCooldown` (`self.AttackSpeed`))
  (`self.TickCooldown`))

(fn `UserConstructionScript`
  (bind _returnvalue (`KismetMathLibrary.Conv_IntToDouble` (+ (* (- (`self.Level`) 1) 200) 300)))
  (`parent.UserConstructionScript`)
  (`CapsuleComponent.SetCapsuleHalfHeight` (`self.Capsule`) _returnvalue true)
  (`CapsuleComponent.SetCapsuleRadius` (`self.Capsule`) _returnvalue true))